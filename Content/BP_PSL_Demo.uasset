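; Demo actor that visualizes live heart-rate data received over MQTT as a beating 3D heart with an HR readout.
; On connect it subscribes to a topic and enters standby with a rotating mesh and blinking label.
; JSON messages start a scale-pulse timeline once, retune its play rate from the first RR interval, and update the HR text.
; EndPlay unsubscribes, resets and disconnects; test events feed sample JSON on timers.
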(event `self.ReceiveBeginPlay`
  ;[0 1 0.4 0.5] Startup Messaging
  (bind _returnvalue (`MQTTSubsystem.GetOrCreateClient_WithProjectURL` null))
  (bind _output_get (set `self.MyClient` _returnvalue))
  (`MQTTClientObject.Connect` _output_get (delegate `OnConnect`)))

(event `HeartbeatStandby`
  ;[1 0 0] Heartbeat
  ;;[1 1 1] Heartbeat Standby
  (`self.HeartbeatReset`)
  (`ActorComponent.Activate` (`self.RotatingMovement`) false)
  (bind _returnvalue (`KismetSystemLibrary.K2_SetTimerDelegate` (delegate `TextRenderBlink`) 0.5 true))
  (set `self.TextRenderVisibilityTimer` _returnvalue))

(event `OnConnect`
  (params (ReturnCode :type "EMQTTConnectReturnCode Enum" :default "Accepted"))
  ;[0 1 0.4 0.5] Startup Messaging
  (switch `EMQTTConnectReturnCode` ReturnCode
    (:`Accepted`
      _)
    (:`AlreadyConnected`
      _))
  (bind _returnvalue (`MQTTClientObject.Subscribe` (`self.MyClient`) (`self.MyTopic`) "ExactlyOnce"))
  (bind _output_get (set `self.MySubscription` _returnvalue))
  (`MQTTSubscriptionObject.SetOnMessageHandler` _output_get (delegate `OnMessage`))
  (`self.HeartbeatStandBy`))

(event `TextRenderBlink`
  ;[1 0 0] Heartbeat
  ;;[1 1 1] Heartbeat Standby
  (bind _isa (`/Engine/EditorBlueprintResources/StandardMacros.FlipFlop`)
    (:`A`
      _)
    (:`B`
      _))
  (`SceneComponent.SetVisibility` (`Actor.RootComponent` (`self.TextRender`)) _isa false))

(event `OnMessage`
  (params (Message :type "MQTTClientMessage Structure (by ref)"))
  ;[0 1 0.4 0.5] Startup Messaging
  (`KismetSystemLibrary.PrintString` (`MQTTSubsystem.GetPayloadString` Message) false)
  (`self.HeartbeatUpdate` (`MQTTSubsystem.GetPayloadJson` (`self.MySubscription`) Message)))

(event `HeartbeatUpdate`
  (params (JsonObject :type "JsonObjectWrapper Structure"))
  ;[1 0 0] Heartbeat
  ;;[1 1 1] Heartbeat Update
  ;;;[0 0.7 1] Field RR: Timeline
  (bind (_outvalue _returnvalue) (`|GetJsonField` JsonObject "rr"))
  (if _returnvalue
    (`|ExecutionSequence`
      (:`then_0`
        (`/Engine/EditorBlueprintResources/StandardMacros.DoOnce` false :!label _label
          (:`Completed`
            (`self.HeartbeatReset`)
            (bind (_direction _alpha) (`Timeline|HeartbeatTimeline` :!via `PlayFromStart`)
              (:`Update`
                (`SceneComponent.SetRelativeScale3D` (`self.HeartMesh`) (`KismetMathLibrary.VLerp` (1.0 1.0 1.0) (2.0 2.0 2.0) _alpha)))))))
      (:`then_1`
        (`TimelineComponent.SetPlayRate` (`self.HeartbeatTimeline`) (/ 1000.0 (`KismetMathLibrary.Conv_IntToDouble` (`|GetArrayItem` _outvalue)))))
      (:`then_2`
        ;;;[0 0.7 1] Field HR
        (bind (_outvalue_2 _returnvalue_2) (`|GetJsonField` JsonObject "hr"))
        (if _returnvalue_2
          (`TextRenderComponent.K2_SetText` (`TextRenderActor.TextRender` (`self.TextRender`)) (`KismetTextLibrary.Conv_IntToText` _outvalue_2)))))))

(event `self.ReceiveEndPlay`
  (params (EndPlayReason :type "EEndPlayReason Enum" :default "Destroyed"))
  (bind _myclient (`self.MyClient`))
  ;[1 0 1 0.5] Teardown Messaging
  (`MQTTClientObject.Unsubscribe` _myclient (`self.MyTopic`))
  (`self.HeartbeatDeactivate`)
  (`MQTTClientObject.Disconnect` _myclient (delegate `OnDisconnect`)))

(event `OnDisconnect`
  ;[1 0 1 0.5] Teardown Messaging
  (`KismetSystemLibrary.PrintString` "MQTT Client disconnected" false))

(event `Testing01`
  ;[1 1 0] Testing
  (`KismetSystemLibrary.K2_SetTimerDelegate` (delegate `Testing02`) 5.0)
  (bind (_outjsonobject _returnvalue) (`JsonBlueprintFunctionLibrary.FromString` "{ \n  \"clientId\": \"MyPSL-01\", \n  \"deviceId\": \"12345678\", \n  \"sessionId\": 1234567890, \n  \"timeStamp\": 1235678901234, \n  \"hr\": 124, \n  \"rr\": [ \n    484, 555 \n  ] \n}"))
  (if _returnvalue
    (`self.HeartbeatUpdate` _outjsonobject)))

(event `HeartbeatDeactivate`
  ;[1 0 0] Heartbeat
  ;;[1 1 1] Heartbeat Deactivate
  (`self.HeartbeatReset`)
  (goto _label :!via `Reset`))

(event `Testing02`
  ;[1 1 0] Testing
  (`KismetSystemLibrary.K2_SetTimerDelegate` (delegate `Testing03`) 5.0)
  (`self.HeartbeatStandBy`))

(event `HeartbeatReset`
  (bind _textrender (`self.TextRender`))
  ;[1 0 0] Heartbeat
  ;;[1 1 1] Helper Event: Heartbeat Reset
  (`TimelineComponent.Stop` (`self.HeartbeatTimeline`))
  (`SceneComponent.SetRelativeScale3D` (`self.HeartMesh`) (1.0 1.0 1.0))
  (`ActorComponent.Deactivate` (`self.RotatingMovement`))
  (`SceneComponent.K2_SetWorldRotation` :`self` (`self.HeartMesh`))
  (`KismetSystemLibrary.K2_ClearAndInvalidateTimerHandle` (`self.TextRenderVisibilityTimer`))
  (`SceneComponent.SetVisibility` (`Actor.RootComponent` _textrender) true false)
  (`TextRenderComponent.K2_SetText` (`TextRenderActor.TextRender` _textrender) "HR"))

(event `Testing03`
  ;[1 1 0] Testing
  (`self.HeartbeatDeactivate`))

(fn `UserConstructionScript`)